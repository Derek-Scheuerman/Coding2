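; BP_Door is a hinged door that opens for a BP_ThirdPersonCharacter holding at least one key and closes behind it.
; Capsule overlap begin and end play a sound and run separate timelines that lerp the hinge's current yaw toward 90 degrees from spawn or back.
; A key is deducted once opening finishes and returned once closing finishes.
; Open and Moving flags gate both events, so overlap changes during movement are ignored.
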(event OnComponentBeginOverlap(Capsule)
  (params (OverlappedComponent :type Primitive%20Component%20Object%20Reference) (OtherActor :type Actor%20Object%20Reference) (OtherComp :type Primitive%20Component%20Object%20Reference) (OtherBodyIndex :type Integer) (bFromSweep :type Boolean) (SweepResult :type Hit%20Result%20Structure%20%28by%20ref%29))
  (bind _hinge (Variables|Default|GetHinge))
  (if (not (Variables|Default|Getopen))
    (if (not (Variables|Default|GetMoving))
      (bind _asbp_third_person_character (Utilities|Casting|CastToBP_ThirdPersonCharacter OtherActor))
      (if (> (Variables|/Game/ThirdPerson/Blueprints/BP_ThirdPersonCharacter.BP_ThirdPersonCharacter_C|GetKeys _asbp_third_person_character) 0)
        (Audio|PlaySoundatLocation "/Game/Audio/Concrete2Steps/concrete2_step-002.concrete2_step-002" (Transformation|GetActorLocation) "0, 0, 0" 1.0 1.0 0.0 0 0 0 0)
        (Variables|Default|SetMoving true)
        (bind _newtrack_0 (Timeline|OpenDoor PlayFromStart)
          (:Update
            (Transformation|SetWorldRotation _hinge (Math|Rotator|MakeRotator 0.0 0.0 (Math|Float|Lerp (.yaw (Transformation|GetWorldRotation _hinge)) (+ (.yaw (Variables|Default|GetSpawn%20Rotation)) 9e+01) _newtrack_0)) false false))
          (:Finished
            (Math|Integer|DecrementInt (Variables|/Game/ThirdPerson/Blueprints/BP_ThirdPersonCharacter.BP_ThirdPersonCharacter_C|GetKeys _asbp_third_person_character)
              (:%20%20
                (Variables|Default|SetMoving false)
                (Variables|Default|Setopen true)))))))))

(event OnComponentEndOverlap(Capsule)
  (params (OverlappedComponent :type Primitive%20Component%20Object%20Reference) (OtherActor :type Actor%20Object%20Reference) (OtherComp :type Primitive%20Component%20Object%20Reference) (OtherBodyIndex :type Integer))
  (bind _hinge (Variables|Default|GetHinge))
  (if (Variables|Default|Getopen)
    (if (not (Variables|Default|GetMoving))
      (bind _asbp_third_person_character (Utilities|Casting|CastToBP_ThirdPersonCharacter OtherActor))
      (Audio|PlaySoundatLocation "/Game/Audio/Concrete2Steps/concrete2_step-002.concrete2_step-002" (Transformation|GetActorLocation) "0, 0, 0" 1.0 1.0 0.0 0 0 0 0)
      (Variables|Default|SetMoving true)
      (bind _newtrack_0 (Timeline|Timeline PlayFromStart)
        (:Update
          (Transformation|SetWorldRotation _hinge (Math|Rotator|MakeRotator 0.0 0.0 (Math|Float|Lerp (.yaw (Transformation|GetWorldRotation _hinge)) (.yaw (Variables|Default|GetSpawn%20Rotation)) _newtrack_0)) false false))
        (:Finished
          (Math|Integer|IncrementInt (Variables|/Game/ThirdPerson/Blueprints/BP_ThirdPersonCharacter.BP_ThirdPersonCharacter_C|GetKeys _asbp_third_person_character)
            (:%20%20
              (Variables|Default|SetMoving false)
              (Variables|Default|Setopen false))))))))

(event EventBeginPlay
  (Variables|Default|SetSpawn%20Rotation (Transformation|GetActorRotation)))

(event Collision|EventActorBeginOverlap
  (params (OtherActor :type Actor%20Object%20Reference)))

(event EventTick
  (params (DeltaSeconds :type Float%20%28single-precision%29)))

(fn ConstructionScript)