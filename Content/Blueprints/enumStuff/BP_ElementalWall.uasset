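; BP_ElementalWall is a barrier that only lets the third-person character pass if it holds the matching elemental type.
; On BeginPlay a TextRender shows the wall's element name as "<Type> barrier".
; On box overlap it searches the character's ElementalType array for its own type, then disables or restores the wall mesh's collision accordingly.
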(event OnComponentBeginOverlap(Box)
  (params (OverlappedComponent :type Primitive%20Component%20Object%20Reference) (OtherActor :type Actor%20Object%20Reference) (OtherComp :type Primitive%20Component%20Object%20Reference) (OtherBodyIndex :type Integer) (bFromSweep :type Boolean) (SweepResult :type Hit%20Result%20Structure%20%28by%20ref%29))
  (bind _thewall (Variables|Default|GetTheWAll))
  (bind _asbp_third_person_character (Utilities|Casting|CastToBP_ThirdPersonCharacter OtherActor))
  (Variables|Default|SetCanPass false)
  (for _array_element (Variables|/Game/ThirdPerson/Blueprints/BP_ThirdPersonCharacter.BP_ThirdPersonCharacter_C|GetElementalType _asbp_third_person_character)
    (if (Utilities|Enum|Equal(Enum) _array_element (Variables|Default|GetElementalType))
      (Variables|Default|SetCanPass true)))
  (if (Variables|Default|GetCanPass)
    (Collision|SetCollisionEnabled _thewall "NoCollision")
    (else
      (Collision|SetCollisionEnabled _thewall "QueryAndPhysics"))))

(event EventBeginPlay
  (Rendering|Components|TextRender|SetText (Variables|Default|GetTextRender) (Utilities|Text|FormatText "{Type} barrier" (Utilities|String|EnumtoString (Variables|Default|GetElementalType)))))

(fn ConstructionScript)