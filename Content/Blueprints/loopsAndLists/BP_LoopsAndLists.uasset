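; BP_LoopsAndLists is a demo actor that prints on-screen text from several loop types when the third-person character overlaps its Sphere.
; The overlap resets a DoN gate and starts DelayLoop, a self-calling event that uses a short Delay and stops when the gate is exhausted.
; Each pass through the gate also fires a self-resetting while countdown, an indexed for loop and a for-each over colors that tint the text.
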(event OnComponentBeginOverlap(Sphere)
  (params (OverlappedComponent :type Primitive%20Component%20Object%20Reference) (OtherActor :type Actor%20Object%20Reference) (OtherComp :type Primitive%20Component%20Object%20Reference) (OtherBodyIndex :type Integer) (bFromSweep :type Boolean) (SweepResult :type Hit%20Result%20Structure%20%28by%20ref%29))
  (Utilities|Casting|CastToBP_ThirdPersonCharacter OtherActor)
  (CallFunction|ResetDelayLoop)
  (CallFunction|DelayLoop))

(event Custom|DelayLoop
  (Development|PrintText (Utilities|Text|FormatText "Loop number: {Count}!" (stale _counter)))
  (Utilities|FlowControl|Delay 0.1)
  (bind _counter (Utilities|FlowControl|DoN 50)
    (:Exit
      (CallFunction|DelayLoop)
      (CallFunction|StartWhileLoop)
      (CallFunction|StartforLoop)
      (CallFunction|StartforEach))))

(event Custom|StartWhileLoop
  (while (> (Variables|Default|GetWhileLoopCounter) 0)
    (Development|PrintText (Utilities|Text|FormatText "There are {uses} more uses in the {loopCount} loop." (Variables|Default|GetWhileLoopCounter) (stale Custom|DelayLoop _counter)) true true "(R=1.000000,G=0.088042,B=0.000000,A=1.000000)")
    (Math|Integer|DecrementInt (Variables|Default|GetWhileLoopCounter)))
  (Variables|Default|SetWhileLoopCounter 10))

(event Custom|StartForLoop
  (for _index (range 0 3)
    (Development|PrintText (Utilities|Text|FormatText "For loop #{index} say hi......" _index) true true "(R=1.000000,G=0.913480,B=0.000000,A=1.000000)")))

(event Custom|StartForEach
  (for (_array_element _array_index) (Utilities|Array|MakeArray "(R=0.184699,G=1.000000,B=0.000000,A=1.000000)" "(R=1.000000,G=0.814551,B=0.000000,A=1.000000)" "(R=1.000000,G=0.000000,B=0.000000,A=1.000000)" "(R=0.000000,G=0.000000,B=1.000000,A=1.000000)")
    (Development|PrintText (Utilities|Text|FormatText "For Each Loop number: {num}" _array_index) true true _array_element)))

(event Custom|ResetDelayLoop
  (Utilities|FlowControl|DoN 50) ; enters at Reset
)

(event EventBeginPlay)

(fn ConstructionScript)