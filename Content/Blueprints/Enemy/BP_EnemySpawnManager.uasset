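; BP_EnemySpawnManager populates the level with BP_AiMoveTo enemies when play begins.
; It finds every BP_EnemySpawnPoint, prints the count, and uses a weighted random roll to spawn an enemy at most of them, owned by that point.
; Each valid spawn gets a random name and mesh material from arrays.
; It then prints the names of all BP_AiMoveTo actors in the level.
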(event EventBeginPlay
  (bind _outactors (Actor|GetAllActorsOfClass "/Game/Blueprints/Enemy/BP_EnemySpawnPoint.BP_EnemySpawnPoint_C"))
  (Development|PrintText (Utilities|Text|FormatText "There are {SpawnPoints} spawn points in the level" (Utilities|Array|Length _outactors)))
  (for _array_element _outactors
    (if (Math|Random|RandomBoolwithWeight 0.75)
      (bind _returnvalue (Game|SpawnActorfromClass "/Game/AI_Blueprints/BP_AiMoveTo.BP_AiMoveTo_C" (Transformation|GetActorTransform _array_element) "Undefined" "MultiplyWithRoot" _array_element 0))
      (if (Utilities|IsValid _returnvalue)
        (Variables|/Game/AI_Blueprints/BP_AiMoveTo.BP_AiMoveTo_C|SetEnemyName _returnvalue (.OutItem (Utilities|Array|Random (Variables|Default|GetEnemyNamesArray))))
        (Rendering|Material|SetMaterial (Variables|/Script/Engine.Character|GetMesh _returnvalue) 0 (.OutItem (Utilities|Array|Random (Variables|Default|GetMaterial)))))))
  (bind _outactors_2 (Actor|GetAllActorsOfClass "/Game/AI_Blueprints/BP_AiMoveTo.BP_AiMoveTo_C"))
  (for _array_element_2 _outactors_2
    (Development|PrintString (Variables|/Game/AI_Blueprints/BP_AiMoveTo.BP_AiMoveTo_C|GetEnemyName _array_element_2))))

(fn ConstructionScript)