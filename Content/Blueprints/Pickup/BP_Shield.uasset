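; BP_Shield is a shield pickup that attaches to a character's skeletal mesh and can be used to block.
; Pickup disables the shield mesh's collision and snaps it to the BPI_ItemSocket socket, while Drop detaches it in world space and restores collision.
; Secondary use toggles the mesh between two relative poses through a FlipFlop and prints a debug "Block" message; primary use is empty.
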(event EventPickup
  (params (SkelitalMesh :type Skeletal%20Mesh%20Component%20Object%20Reference))
  (Collision|SetCollisionEnabled (Variables|Default|GetSheildMesh) "NoCollision")
  (Transformation|AttachComponentToComponent SkelitalMesh "BPI_ItemSocket" "SnapToTarget" "SnapToTarget" "KeepRelative" true))

(event EventDrop
  (params (SkelMesh :type Skeletal%20Mesh%20Component%20Object%20Reference))
  (Transformation|DetachFromActor "KeepWorld" "KeepWorld" "KeepRelative")
  (Collision|SetCollisionEnabled (Variables|Default|GetSheildMesh) "QueryAndPhysics"))

(event EventUseSecondary
  (bind _sheildmesh (Variables|Default|GetSheildMesh))
  (Development|PrintString "Block")
  (Utilities|FlowControl|FlipFlop
    (:A
      (Transformation|SetRelativeLocationAndRotation _sheildmesh "20.000000,0.000000,0.000000" "90.000000,0.000000,90.000000" false true))
    (:B
      (Transformation|SetRelativeLocationAndRotation _sheildmesh "0.000000,0.000000,-20.000000" "0.000000,0.000000,80.000000" false true))))

(event EventUsePrimary)

(fn ConstructionScript)