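; BP_MachineGun is a pickup weapon that attaches to the player's GunSocket as a right-hand item and fires projectiles.
; Pickup and Drop toggle the body's physics and collision while attaching or detaching it.
; UsePrimary spends player stamina if enough remains, then plays a gunplay montage.
; The montage notify plays a water-gun sound, spawns BP_Projectile at the barrel and propels it along the camera's direction.
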(event EventPickup
  (params (SkelitalMesh :type Skeletal%20Mesh%20Component%20Object%20Reference) (PlayerRef :type BP%20Third%20Person%20Character%20Object%20Reference))
  (bind _machinegunbody (Variables|Default|GetMachineGunBody))
  (Variables|Default|SetPlayer%20Ref PlayerRef)
  (Physics|SetSimulatePhysics _machinegunbody false)
  (Collision|SetCollisionEnabled _machinegunbody "NoCollision")
  (Transformation|AttachComponentToComponent SkelitalMesh "GunSocket" "SnapToTarget" "SnapToTarget" "SnapToTarget" true))

(event EventDrop
  (bind _machinegunbody (Variables|Default|GetMachineGunBody))
  (Transformation|DetachFromActor "KeepWorld" "KeepWorld" "KeepRelative")
  (Collision|SetCollisionEnabled _machinegunbody "QueryAndPhysics")
  (Physics|SetSimulatePhysics _machinegunbody true))

(event EventUsePrimary
  (bind _player_ref (Variables|Default|GetPlayer%20Ref))
  (if (not (< (- (Variables|/Game/ThirdPerson/Blueprints/BP_ThirdPersonCharacter.BP_ThirdPersonCharacter_C|GetStamina (Variables|Default|GetPlayer%20Ref)) 4.0) 0.0))
    (Variables|/Game/ThirdPerson/Blueprints/BP_ThirdPersonCharacter.BP_ThirdPersonCharacter_C|SetStamina _player_ref (- (Variables|/Game/ThirdPerson/Blueprints/BP_ThirdPersonCharacter.BP_ThirdPersonCharacter_C|GetStamina (Variables|Default|GetPlayer%20Ref)) 4.0))
    (Default|StaminaCheck _player_ref)
    (Variables|/Game/ThirdPerson/Blueprints/BP_ThirdPersonCharacter.BP_ThirdPersonCharacter_C|SetIsAttacking _player_ref true)
    (Animation|Montage|PlayMontage (Variables|/Script/Engine.Character|GetMesh _player_ref) "/Game/ThirdPerson/Gunplay_Montage.Gunplay_Montage" 1.0 0.0 "None" false
      (:OnNotifyBegin
        (Audio|PlaySoundatLocation "/Game/Audio/Concrete2Steps/WaterGun.WaterGun" (Transformation|GetActorLocation) "0, 0, 0" 1.0 1.0 0.0 0 0 0 0)
        (bind _returnvalue (Game|SpawnActorfromClass "/Game/Blueprints/BP_Projectile.BP_Projectile_C" (Transformation|GetWorldTransform (Variables|Default|GetBarrel)) "AlwaysSpawn" "MultiplyWithRoot" 0 0)) ; Spawn the bullet above the player's head
        (Physics|AddForce (Variables|/Game/Blueprints/BP_Projectile.BP_Projectile_C|GetSphere _returnvalue) (* (Camera|GetCameraRotation (Game|GetPlayerCameraManager 0)) 2e+05) "None" true) ; Shoot the bullet in the camera's direction
        (Variables|/Game/ThirdPerson/Blueprints/BP_ThirdPersonCharacter.BP_ThirdPersonCharacter_C|SetIsAttacking (Variables|Default|GetPlayer%20Ref) false)))))

(fn ConstructionScript)

(fn RightHand?
  (return true))