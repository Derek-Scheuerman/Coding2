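; BP_HealthPotion is a left-hand pickup item that restores some of the player's health when used.
; Pickup stores the player reference, disables the mesh's physics and collision and snaps it to the skeletal mesh's left weapon socket, while Drop detaches it and re-enables both.
; UseSecondary applies the heal, clears the holding flag for the hand reported by RightHand, which always returns false, then destroys the potion.
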(event EventUseSecondary
  (bind _player_ref (Variables|Default|GetPlayer%20Ref))
  (Default|ChangeHealth _player_ref 0.3)
  (bind _righthand_ (CallFunction|RightHand?))
  (if _righthand_
    (Variables|/Game/ThirdPerson/Blueprints/BP_ThirdPersonCharacter.BP_ThirdPersonCharacter_C|SetisHoldingItemRight _player_ref false)
    (else
      (Variables|/Game/ThirdPerson/Blueprints/BP_ThirdPersonCharacter.BP_ThirdPersonCharacter_C|SetisHoldingItemLeft _player_ref false)))
  (Actor|DestroyActor))

(event EventDrop
  (bind _healthmesh (Variables|Default|GetHealthMesh))
  (Transformation|DetachFromActor "KeepWorld" "KeepWorld" "KeepRelative")
  (Collision|SetCollisionEnabled _healthmesh "QueryAndPhysics")
  (Physics|SetSimulatePhysics _healthmesh true))

(event EventPickup
  (params (SkelitalMesh :type Skeletal%20Mesh%20Component%20Object%20Reference) (PlayerRef :type BP%20Third%20Person%20Character%20Object%20Reference))
  (bind _healthmesh (Variables|Default|GetHealthMesh))
  ;[0.15 0.15 0.15 0.5] Pickup Function
  (Variables|Default|SetPlayer%20Ref PlayerRef)
  (Development|PrintText (Utilities|Text|FormatText "{name} is getting picked up and attached to {mesh}." (Utilities|String|MakeLiteralString "HealthPotion") SkelitalMesh) true true "(R=1.000000,G=0.174349,B=0.977565,A=1.000000)")
  (Physics|SetSimulatePhysics _healthmesh false)
  (Collision|SetCollisionEnabled _healthmesh "NoCollision")
  (Transformation|AttachComponentToComponent SkelitalMesh "Weapon_L_S" "SnapToTarget" "SnapToTarget" "KeepWorld" true))

(fn ConstructionScript)

(fn RightHand?
  (return false))